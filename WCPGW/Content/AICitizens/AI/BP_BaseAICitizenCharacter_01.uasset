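; Base AI citizen character that gets a random skeletal mesh at construction and spawns its default controller on BeginPlay.
; Death ragdolls it, stops movement and, once per death, registers it as a patient with SimpleGamemode after a short delay; Revived restores walking and resets that gate.
; A motion controller can pick it up and drop it via physics toggling and attachment.
; Slot montage playback tracks a playing flag with a timer.
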(event Custom|CallAmbulance
  (Utilities|FlowControl|DoOnce false
    (:Completed
      (Utilities|FlowControl|Delay 3.0)
      (Default|AddPatient (.AsSimple%20Gamemode (Utilities|Casting|CastToSimpleGamemode (Game|GetGameMode))) self))))

(event Custom|Revived
  (Pawn|Components|CharacterMovement|SetMovementMode (Variables|Character|GetCharacterMovement) "MOVE_Walking" 0)
  (Development|PrintString "Back from the deaad")
  (Physics|SetSimulatePhysics (Variables|Character|GetMesh) false)
  (Utilities|FlowControl|DoOnce false) ; enters at Reset
)

(event EventBeginPlay
  (Pawn|SpawnDefaultController))

(event EventPickup
  (params (AttachTo :type Scene%20Component%20Object%20Reference))
  ;[1 1 1] Pick Up and Drop Civilian
  (Physics|SetSimulatePhysics (Variables|Character|GetMesh) true)
  (Transformation|AttachComponentToComponent (VehicleSound|GetRootComponent) AttachTo "None" "KeepWorld" "KeepWorld" "KeepWorld" false))

(event EventDrop
  ;[1 1 1] Pick Up and Drop Civilian
  (Physics|SetSimulatePhysics (Variables|Character|GetMesh) false)
  (Transformation|DetachFromActor "KeepWorld" "KeepWorld" "KeepWorld"))

(fn ConstructionScript
  (CallFunction|RandomMesh))

(fn PlaySlotAnimation
  (params (Animation :type Anim%20Montage%20Object%20Reference))
  (Variables|Default|SetbIsPlayingAnimation true)
  (bind _returnvalue (Animation|PlayAnimMontage Animation 1.0 "None"))
  (Utilities|Time|SetTimerbyFunctionName 0 "OnAnimationFinished" _returnvalue))

(fn OnAnimationFinished
  (Variables|Default|SetbIsPlayingAnimation false))

(fn IsPlayingSlotAnimation
  (return (Variables|Default|GetbIsPlayingAnimation)))

(fn RandomMesh
  (bind _mesh (Variables|Character|GetMesh))
  (switch int (Math|Random|RandomIntegerinRange 0 18)
    (:0
      (Class|SkinnedMeshComponent|SetSkeletalMesh _mesh "/Game/SimpleStuff/SimplePeople/Characters/SK_Character_BeachBabe.SK_Character_BeachBabe" true))
    (:1
      (Class|SkinnedMeshComponent|SetSkeletalMesh _mesh "/Game/SimpleStuff/SimplePeople/Characters/SK_Character_BusinessMan.SK_Character_BusinessMan" true))
    (:2
      (Class|SkinnedMeshComponent|SetSkeletalMesh _mesh "/Game/SimpleStuff/SimplePeople/Characters/SK_Character_Doctor.SK_Character_Doctor" true))
    (:3
      (Class|SkinnedMeshComponent|SetSkeletalMesh _mesh "/Game/SimpleStuff/SimplePeople/Characters/SK_Character_FireFighter.SK_Character_FireFighter" true))
    (:4
      (Class|SkinnedMeshComponent|SetSkeletalMesh _mesh "/Game/SimpleStuff/SimplePeople/Characters/SK_Character_Hobo.SK_Character_Hobo" true))
    (:5
      (Class|SkinnedMeshComponent|SetSkeletalMesh _mesh "/Game/SimpleStuff/SimplePeople/Characters/SK_Character_HouseWifey.SK_Character_HouseWifey" true))
    (:6
      (Class|SkinnedMeshComponent|SetSkeletalMesh _mesh "/Game/SimpleStuff/SimplePeople/Characters/SK_Character_Pimp.SK_Character_Pimp" true))
    (:7
      (Class|SkinnedMeshComponent|SetSkeletalMesh _mesh "/Game/SimpleStuff/SimplePeople/Characters/SK_Character_Policeman.SK_Character_Policeman" true))
    (:8
      (Class|SkinnedMeshComponent|SetSkeletalMesh _mesh "/Game/SimpleStuff/SimplePeople/Characters/SK_Character_Prostitute.SK_Character_Prostitute" true))
    (:9
      (Class|SkinnedMeshComponent|SetSkeletalMesh _mesh "/Game/SimpleStuff/SimplePeople/Characters/SK_Character_Punk.SK_Character_Punk" true))
    (:10
      (Class|SkinnedMeshComponent|SetSkeletalMesh _mesh "/Game/SimpleStuff/SimplePeople/Characters/SK_Character_RiotCop.SK_Character_RiotCop" true))
    (:11
      (Class|SkinnedMeshComponent|SetSkeletalMesh _mesh "/Game/SimpleStuff/SimplePeople/Characters/SK_Character_Roadworker.SK_Character_Roadworker" true))
    (:12
      (Class|SkinnedMeshComponent|SetSkeletalMesh _mesh "/Game/SimpleStuff/SimplePeople/Characters/SK_Character_Robber.SK_Character_Robber" true))
    (:13
      (Class|SkinnedMeshComponent|SetSkeletalMesh _mesh "/Game/SimpleStuff/SimplePeople/Characters/SK_Character_Hobo.SK_Character_Hobo" true))
    (:14
      (Class|SkinnedMeshComponent|SetSkeletalMesh _mesh "/Game/SimpleStuff/SimplePeople/Characters/SK_Character_Sheriff.SK_Character_Sheriff" true))
    (:15
      (Class|SkinnedMeshComponent|SetSkeletalMesh _mesh "/Game/SimpleStuff/SimplePeople/Characters/SK_Character_Streetman.SK_Character_Streetman" true))
    (:16
      (Class|SkinnedMeshComponent|SetSkeletalMesh _mesh "/Game/SimpleStuff/SimplePeople/Characters/SK_Character_Policeman.SK_Character_Policeman" true))
    (:17
      (Class|SkinnedMeshComponent|SetSkeletalMesh _mesh "/Game/SimpleStuff/SimplePeople/Characters/SK_Character_Trucker.SK_Character_Trucker" true))
    (:18
      (Class|SkinnedMeshComponent|SetSkeletalMesh _mesh "/Game/SimpleStuff/SimplePeople/Characters/SK_Character_Waitress.SK_Character_Waitress" true))))

(fn Death-Ragdoll
  (Physics|SetSimulatePhysics (Variables|Character|GetMesh) true)
  (Pawn|Components|CharacterMovement|DisableMovement (Variables|Character|GetCharacterMovement))
  (CallFunction|CallAmbulance))