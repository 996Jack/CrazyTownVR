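; Animated skeletal mesh actor for AI citizens that continuously plays randomly chosen animations.
; On BeginPlay it sums the play chances of all AnimationsToPlay entries, then starts the first animation.
; GetAnimation does a weighted random pick by accumulating chances against a random value within that total.
; Each animation plays once without looping, and a timer set to its play length calls AnimationFinished to pick the next.
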(event EventBeginPlay
  (for _array_element (Variables|Default|GetAnimationsToPlay)
    (Variables|Default|SetSummaryAnimationChance (+ (.playchance _array_element) (Variables|Default|GetSummaryAnimationChance))))
  (CallFunction|PlayRandomAnimation))

(fn ConstructionScript)

(fn GetAnimation
  (LocalVariables|SetRandomChance (Math|Random|RandomFloatinRange 0.0 (Variables|Default|GetSummaryAnimationChance)))
  (for _array_element (Variables|Default|GetAnimationsToPlay)
    (bind _output_get (LocalVariables|SetActualChance (+ (.playchance _array_element) (LocalVariables|GetActualChance))))
    (if (> _output_get (LocalVariables|GetRandomChance))
      (return (.animation _array_element))))
  (return 0))

(fn PlayRandomAnimation
  (bind _animation (CallFunction|GetAnimation))
  (Components|Animation|PlayAnimation (Variables|Default|GetSkeletalMesh) _animation false)
  (bind _returnvalue (Animation|GetPlayLength _animation))
  (Utilities|Time|SetTimerbyFunctionName 0 "AnimationFinished" _returnvalue))

(fn AnimationFinished
  (CallFunction|PlayRandomAnimation))