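; Citizen generator that populates an area with AI citizens when play begins.
; It spawns a set number of actors, each of a random class from the citizen template list, with random yaw.
; Spawn positions come from random points in the SpawnArea box, projected onto the navmesh and raised above it.
; Logic for randomly coloring mannequin body and logo materials is present but disconnected, so it never runs.
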(event EventBeginPlay
  (bind _spawnarea (Variables|Default|GetSpawnArea))
  (bind _citizenstemplates (Variables|Default|GetCitizensTemplates))
  (bind _returnvalue (Transformation|GetWorldLocation _spawnarea))
  (bind _returnvalue_2 (Components|Box|GetScaledBoxExtent _spawnarea))
  (bind _returnvalue_3 (Math|Random|RandomPointinBoundingBox _returnvalue _returnvalue_2))
  (bind _projectedlocation (AI|Navigation|ProjectPointtoNavigation _returnvalue_3 0 "/Script/NavigationSystem.RecastFilter_UseDefaultArea" "2048.000000,2048.000000,2048.000000"))
  (bind (_x _y _z) (Math|Vector|BreakVector _projectedlocation))
  ;[1 1 1] Spawn citizens
  (for _index (range 1 (Variables|Default|GetCitizensToSpawn))
    (bind _returnvalue_4 (Game|SpawnActorfromClass (Utilities|Array|Get(acopy) _citizenstemplates (Math|Random|RandomInteger (Utilities|Array|Length _citizenstemplates))) (Math|Transform|MakeTransform (Math|Vector|MakeVector _x _y (+ _z 1.8e+02)) (Math|Rotator|MakeRotator 0.0 0.0 (Math|Random|RandomFloatinRange 0.0 359.0)) "1,1,1") "AlwaysSpawn" 0 0))
    (Utilities|IsValid _returnvalue_4)))

(fn ConstructionScript)